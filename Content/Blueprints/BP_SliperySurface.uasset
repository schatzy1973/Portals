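; BP_SliperySurface is a trigger volume that makes BP_FirstPersonCharacter slide as if on ice.
; Entering the Box overrides the character's ground friction, walking braking deceleration and max walk speed with ice variables.
; Leaving waits for a Duration delay, then sets each value once to a Lerp between its ice value and a hardcoded normal value, using a fixed Alpha variable rather than a gradual blend.
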(event OnComponentBeginOverlap(Box)
  (params (OverlappedComponent :type Primitive%20Component%20Object%20Reference) (OtherActor :type Actor%20Object%20Reference) (OtherComp :type Primitive%20Component%20Object%20Reference) (OtherBodyIndex :type Integer) (bFromSweep :type Boolean) (SweepResult :type Hit%20Result%20Structure%20%28by%20ref%29))
  (bind _asbp_first_person_character (Utilities|Casting|CastToBP_FirstPersonCharacter OtherActor))
  (Variables|/Script/Engine.CharacterMovementComponent|SetGroundFriction (Variables|/Script/Engine.Character|GetCharacterMovement _asbp_first_person_character) (Variables|Default|GetIce%20Ground%20Friction))
  (Variables|/Script/Engine.CharacterMovementComponent|SetBrakingDecelerationWalking (Variables|/Script/Engine.Character|GetCharacterMovement _asbp_first_person_character) (Variables|Default|GetIce%20Braking%20Deceleration%20Walking))
  (Variables|/Script/Engine.CharacterMovementComponent|SetMaxWalkSpeed (Variables|/Script/Engine.Character|GetCharacterMovement _asbp_first_person_character) (Variables|Default|GetMax%20Walk%20Speed)))

(event OnComponentEndOverlap(Box)
  (params (OverlappedComponent :type Primitive%20Component%20Object%20Reference) (OtherActor :type Actor%20Object%20Reference) (OtherComp :type Primitive%20Component%20Object%20Reference) (OtherBodyIndex :type Integer))
  (bind _alpha (Variables|Default|GetAlpha))
  (bind _asbp_first_person_character (Utilities|Casting|CastToBP_FirstPersonCharacter OtherActor))
  (Utilities|FlowControl|Delay (Variables|Default|GetDuration))
  (Variables|/Script/Engine.CharacterMovementComponent|SetGroundFriction (Variables|/Script/Engine.Character|GetCharacterMovement _asbp_first_person_character) (Math|Float|Lerp (Variables|Default|GetIce%20Ground%20Friction) 8.0 _alpha))
  (Variables|/Script/Engine.CharacterMovementComponent|SetBrakingDecelerationWalking (Variables|/Script/Engine.Character|GetCharacterMovement _asbp_first_person_character) (Math|Float|Lerp (Variables|Default|GetIce%20Braking%20Deceleration%20Walking) 2048.0 _alpha))
  (Variables|/Script/Engine.CharacterMovementComponent|SetMaxWalkSpeed (Variables|/Script/Engine.Character|GetCharacterMovement _asbp_first_person_character) (Math|Float|Lerp (Variables|Default|GetMax%20Walk%20Speed) 6e+02 _alpha)))

(event EventBeginPlay)

(event Collision|EventActorBeginOverlap
  (params (OtherActor :type Actor%20Object%20Reference)))

(event EventTick
  (params (DeltaSeconds :type Float%20%28single-precision%29)))

(fn ConstructionScript)