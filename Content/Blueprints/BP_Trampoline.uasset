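; BP_Trampoline is a trampoline actor that bounces the first-person character upward when it overlaps the Colision component.
; The launch overrides vertical velocity with the character's negated Z speed plus LaunchVelocityZ, so faster falls give stronger bounces.
; A DoOnce gate blocks repeat launches, resetting after a Duration delay following a launch or an end overlap.
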(event OnComponentBeginOverlap(Colision)
  (params (OverlappedComponent :type Primitive%20Component%20Object%20Reference) (OtherActor :type Actor%20Object%20Reference) (OtherComp :type Primitive%20Component%20Object%20Reference) (OtherBodyIndex :type Integer) (bFromSweep :type Boolean) (SweepResult :type Hit%20Result%20Structure%20%28by%20ref%29))
  (Utilities|FlowControl|DoOnce false :!label _label
    (:Completed
      (bind _asbp_first_person_character (Utilities|Casting|CastToBP_FirstPersonCharacter OtherActor))
      (Utilities|IsValid _asbp_first_person_character
        (:Is%20Valid
          (Character|LaunchCharacter _asbp_first_person_character (Math|Vector|MakeVector 0.0 0.0 (+ (* (.z (Transformation|GetVelocity _asbp_first_person_character)) -1.0) (Variables|Default|GetLaunch%20Velocity%20Z))) false true)
          (Utilities|FlowControl|Delay (Variables|Default|GetDuration))
          (goto _label Reset))))))

(event OnComponentEndOverlap(Colision)
  (params (OverlappedComponent :type Primitive%20Component%20Object%20Reference) (OtherActor :type Actor%20Object%20Reference) (OtherComp :type Primitive%20Component%20Object%20Reference) (OtherBodyIndex :type Integer))
  (Utilities|FlowControl|Delay (Variables|Default|GetDuration))
  (Utilities|FlowControl|DoOnce false) ; enters at Reset
)

(event EventBeginPlay)

(event Collision|EventActorBeginOverlap
  (params (OtherActor :type Actor%20Object%20Reference)))

(event EventTick
  (params (DeltaSeconds :type Float%20%28single-precision%29)))

(fn ConstructionScript)