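; BP_Note is a level design kit Blueprint that displays an in-world text note with a headline and four lines of text.
; Its construction script copies the Headline and TextLine variables into matching TextRender components, so the note updates whenever construction reruns.
; The event graph holds only disabled default events, so it adds no runtime behavior.
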(event EventBeginPlay)

(event Collision|EventActorBeginOverlap
  (params (OtherActor :type Actor%20Object%20Reference)))

(event EventTick
  (params (DeltaSeconds :type Float%20%28single-precision%29)))

(fn ConstructionScript
  (Rendering|Components|TextRender|SetText (Variables|Default|GetTextRender%20-%20Headline) (Variables|Default|GetHeadline))
  (Rendering|Components|TextRender|SetText (Variables|Default|GetTextRender%20-%20Line_01) (Variables|Default|GetText_Line_01))
  (Rendering|Components|TextRender|SetText (Variables|Default|GetTextRender%20-%20Line_02) (Variables|Default|GetText_Line_02))
  (Rendering|Components|TextRender|SetText (Variables|Default|GetTextRender%20-%20Line_03) (Variables|Default|GetText_Line_03))
  (Rendering|Components|TextRender|SetText (Variables|Default|GetTextRender%20-%20Line_04) (Variables|Default|GetText_Line_04)))