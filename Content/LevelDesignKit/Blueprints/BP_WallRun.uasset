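; BP_WallRun is a level design kit actor that teleports the player through two trigger volumes, one for each side.
; Overlapping TV_Swing_Right or TV_Swing_Left calls the matching function, which moves player character 0 to the location and rotation of TPRight or TPLeft.
; The overlapping actor is not checked, and the Blueprint holds no wall-running movement logic.
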(event OnComponentBeginOverlap(TV_Swing_Right)
  (params (OverlappedComponent :type Primitive%20Component%20Object%20Reference) (OtherActor :type Actor%20Object%20Reference) (OtherComp :type Primitive%20Component%20Object%20Reference) (OtherBodyIndex :type Integer) (bFromSweep :type Boolean) (SweepResult :type Hit%20Result%20Structure%20%28by%20ref%29))
  (|TeleportPlayerstotheRight))

(event OnComponentBeginOverlap(TV_Swing_Left)
  (params (OverlappedComponent :type Primitive%20Component%20Object%20Reference) (OtherActor :type Actor%20Object%20Reference) (OtherComp :type Primitive%20Component%20Object%20Reference) (OtherBodyIndex :type Integer) (bFromSweep :type Boolean) (SweepResult :type Hit%20Result%20Structure%20%28by%20ref%29))
  (|TeleportPlayerstotheLeft))

(fn ConstructionScript)