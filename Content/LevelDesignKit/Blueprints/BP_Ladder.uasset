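; BP_Ladder is a level design kit ladder that moves the player by teleport instead of climbing, in 2m or 4m variants chosen by TallLadder.
; The construction script hides and disables collision on the unused variant, and BeginPlay enables the active top trigger volume.
; Overlapping the bottom or top volume teleports player character 0 to the opposite end's marker, without checking which actor overlapped.
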(event OnComponentBeginOverlap(TV_Ladder_Bottom)
  (params (OverlappedComponent :type Primitive%20Component%20Object%20Reference) (OtherActor :type Actor%20Object%20Reference) (OtherComp :type Primitive%20Component%20Object%20Reference) (OtherBodyIndex :type Integer) (bFromSweep :type Boolean) (SweepResult :type Hit%20Result%20Structure%20%28by%20ref%29))
  ;[1 1 1] Checks which ladder is in use, then teleport
  (if (Variables|LadderHeight|GetTall_Ladder)
    (|TeleportPlayer4mLadder)
    (else
      (|TeleportPlayer2mLadder))))

(event OnComponentBeginOverlap(TV_Ladder_4m)
  (params (OverlappedComponent :type Primitive%20Component%20Object%20Reference) (OtherActor :type Actor%20Object%20Reference) (OtherComp :type Primitive%20Component%20Object%20Reference) (OtherBodyIndex :type Integer) (bFromSweep :type Boolean) (SweepResult :type Hit%20Result%20Structure%20%28by%20ref%29))
  ;[1 1 1] 4m Ladder teleports to Bottom
  (|TeleportPlayerBottomOfLadder4m))

(event OnComponentBeginOverlap(TV_Ladder_2m)
  (params (OverlappedComponent :type Primitive%20Component%20Object%20Reference) (OtherActor :type Actor%20Object%20Reference) (OtherComp :type Primitive%20Component%20Object%20Reference) (OtherBodyIndex :type Integer) (bFromSweep :type Boolean) (SweepResult :type Hit%20Result%20Structure%20%28by%20ref%29))
  ;[1 1 1] 2m Ladder teleports to Bottom
  (|TeleportPlayerBottomOfLadder2m))

(event EventBeginPlay
  ;[1 1 1] Set Correct Teleport Triggers
  (if (Variables|LadderHeight|GetTall_Ladder)
    (|4mTeleportVolEnabled)
    (else
      (|2mTeleportVolEnabled))))

(fn ConstructionScript
  ;[1 1 1] Setting Up Ladder Variation
  (if (Variables|LadderHeight|GetTall_Ladder)
    (|HideLadder2m_2)
    (else
      (|Hide4mLadder_2))))